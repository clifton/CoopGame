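; BP_ExplodingBarrel is a destructible barrel that explodes when its health component reports death.
; On BeginPlay it binds to HealthComp's OnDeath event.
; The explosion swaps the mesh to an exploded material, launches it upward with a randomized velocity impulse, and fires the RadialForce impulse.
; It then applies radial damage with distance falloff around the barrel, passing along the instigator who triggered the death.
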(event Custom|BarrelExplode
  (params (HealthComp :type S%20Health%20Component%20Object%20Reference) (Health :type Float%20%28single-precision%29) (HealthDelta :type Float%20%28single-precision%29) (DamageType :type Damage%20Type%20Object%20Reference) (InstigatedBy :type Controller%20Object%20Reference) (DamageCauser :type Actor%20Object%20Reference))
  (bind _meshcomp (Variables|Default|GetMeshComp))
  (Rendering|Material|SetMaterial _meshcomp 0 "/Game/Challenges/ExplosiveBarrel/M_ExplosiveBarrelExploded.M_ExplosiveBarrelExploded")
  (Physics|AddImpulse _meshcomp (Math|Vector|MakeVector (Math|Random|RandomFloatinRange 0.0 3e+02) (Math|Random|RandomFloatinRange 0.0 3e+02) 4e+02) "None" true)
  (Class|RadialForceComponent|FireImpulse (Variables|Default|GetRadialForce))
  (Class|GameplayStatics|ApplyRadialDamagewithFalloff 2e+02 5.0 (Transformation|GetActorLocation) 1e+02 5e+02 1.0 0 0 (Components|GetOwner (Variables|Default|GetMeshComp)) InstigatedBy "ECC_GameTraceChannel1"))

(event EventBeginPlay
  (EventDispatchers|AssignOnDeath (Variables|Default|GetHealthComp) (delegate Custom|BarrelExplode)))

(event Collision|EventActorBeginOverlap
  (params (OtherActor :type Actor%20Object%20Reference)))

(event EventTick
  (params (DeltaSeconds :type Float%20%28single-precision%29)))

(fn ConstructionScript)