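; Player pawn Blueprint for the coop game that sets up the local player's HUD and handles weapon switching.
; On BeginPlay it adds crosshair and health indicator widgets, and Tick prints HealthComp health as debug text, both only when locally controlled.
; SelectWeapon ignores a matching class, otherwise detaches the current weapon without destroying it, then spawns the new one and snaps it to the mesh's WeaponSocket.
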(event EventBeginPlay
  (if (Pawn|IsLocallyControlled)
    (Utilities|FlowControl|Sequence
      (:then_0
        (bind _returnvalue (UserInterface|CreateWidget "/Game/CoopGame/UI/WBP_Crosshair.WBP_Crosshair_C"))
        (UserInterface|Viewport|AddtoViewport _returnvalue 0))
      (:then_1
        (bind _returnvalue_2 (UserInterface|CreateWidget "/Game/CoopGame/UI/WBP_HealthIndicator.WBP_HealthIndicator_C"))
        (UserInterface|Viewport|AddtoViewport _returnvalue_2 0)))))

(event EventTick
  (params (DeltaSeconds :type Float%20%28single-precision%29))
  (if (Pawn|IsLocallyControlled)
    (Development|PrintString (Utilities|String|ToString(Float) (Variables|/Script/CoopGame.SHealthComponent|GetHealth (Variables|Default|GetHealthComp))) true true "(R=0.000000,G=0.406250,B=0.072587,A=1.000000)" 0.0)))

(fn ConstructionScript)

(fn SelectWeapon
  (params (WeaponClass :type S%20Weapon%20Class%20Reference))
  (if (== (Utilities|GetClass (Variables|Default|GetCurrentWeapon_0)) WeaponClass)
    (return)
    (else
      (Utilities|IsValid (Variables|Default|GetCurrentWeapon_0)
        (:Is%20Valid
          (Transformation|DetachFromActor (Variables|Default|GetCurrentWeapon_0) "KeepRelative" "KeepRelative" "KeepRelative"))
        (:Is%20Not%20Valid
          _))
      (bind _returnvalue (Game|SpawnActorfromClass WeaponClass (Math|Transform|MakeTransform "0, 0, 0") "AlwaysSpawn" self 0))
      (bind _output_get (Variables|Default|SetCurrentWeapon_0 _returnvalue))
      (Transformation|AttachComponentToComponent _output_get (Variables|Character|GetMesh) "WeaponSocket" "SnapToTarget" "SnapToTarget" "SnapToTarget" true)
      (return))))